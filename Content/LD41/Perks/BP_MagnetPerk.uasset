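; BP_MagnetPerk is a car perk that, when consumed, teleports the consuming car to the closest other car.
; Consume runs MagnetClosestCar, then hands off to the parent perk's Consume.
; The search scans all car actors, skipping the user and tightening MinDistance to each nearer match, so its starting value caps the range.
; Car.Teleport is called only when a valid target is found.
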(event `self.Consume`
  (params (Car :type "Car Object Reference"))
  (`self.MagnetClosestCar` Car)
  (`parent.Consume` Car))

(fn `MagnetClosestCar`
  (params (Car :type "Car Object Reference"))
  (locals (ClosestCar :type "Car Object Reference") (MinDistance :type "Float (double-precision)" :default 100000000.0))
  (bind _closestcar (`local.ClosestCar`))
  (bind _outactors (`GameplayStatics.GetAllActorsOfClass` "/Script/LD41.Car"))
  (for _array_element _outactors
    (bind _returnvalue (`Actor.GetDistanceTo` _array_element Car))
    (if (and (!= _array_element Car) (<= _returnvalue (`local.MinDistance`)))
      (set `local.ClosestCar` _array_element)
      (set `local.MinDistance` _returnvalue)))
  (`/Engine/EditorBlueprintResources/StandardMacros.IsValid` _closestcar
    (:`Is Valid`
      (`Car.Teleport` Car _closestcar))))
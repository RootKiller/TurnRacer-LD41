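; AI controller for a computer-driven car that extends its parent's Think logic with automatic perk use.
; Each Think runs the parent behavior, then ConsumePerks tries a petrol perk when fuel is low.
; Failing that, it tries a magnet perk if the opponent is in front, tested by a dot product with the car's forward vector.
; The opponent is simply the first other Car actor found in the world.
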(event `self.Think`
  (`parent.Think`)
  (`self.ConsumePerks`))

(fn `ConsumePerks`
  (bind _car (`self.GetOpponentCar`))
  (bind _returnvalue (`self.GetCar`))
  (`/Engine/EditorBlueprintResources/StandardMacros.IsValid` _returnvalue
    (:`Is Valid`
      (`|ExecutionSequence`
        (:`then_0`
          (if (<= (`Car.Fuel` _returnvalue) 10)
            (bind _returnvalue_2 (`Car.ConsumePerkOfClass` _returnvalue "/Game/LD41/Perks/BP_PetrolPerk.BP_PetrolPerk_C"))
            (if _returnvalue_2
              (return))))
        (:`then_1`
          (`/Engine/EditorBlueprintResources/StandardMacros.IsValid` _car
            (:`Is Valid`
              (if (> (`KismetMathLibrary.Dot_VectorVector` (`KismetMathLibrary.Normal` (- (`self.K2_GetActorLocation` _car) (`self.K2_GetActorLocation` _returnvalue))) (`self.GetActorForwardVector` _returnvalue)) 0.0)
                (bind _returnvalue_3 (`Car.ConsumePerkOfClass` _returnvalue "/Game/LD41/Perks/BP_MagnetPerk.BP_MagnetPerk_C"))
                (if _returnvalue_3
                  (return))))))))))

(fn `GetOpponentCar`
  (returns (Car :type "Car Object Reference"))
  (bind _outactors (`GameplayStatics.GetAllActorsOfClass` "/Script/LD41.Car"))
  (for _array_element _outactors
    (if (!= _array_element (`self.GetCar`))
      (return _array_element))))

(fn `UserConstructionScript`)
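; An asphalt-with-walls track prefab for the LD41 race tracks that varies where its barrel obstacle sits.
; On BeginPlay it runs the parent logic, then sets a random boolean that picks one of two marker components, CubeLocationA or CubeLocationB.
; The Barrels component moves to that marker's world transform without sweeping.
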(event `self.ReceiveBeginPlay`
  (`parent.ReceiveBeginPlay`)
  (set `self.CubeLocation` (`KismetMathLibrary.RandomBool`))
  (bind _transform (`self.GetBarrelTransform`))
  (`SceneComponent.K2_SetWorldTransform` (`self.Barrels`) _transform false false))

(fn `GetBarrelTransform`
  (returns (Transform :type "Transform Structure"))
  (return (`SceneComponent.K2_GetComponentToWorld` (select `bool` (`self.CubeLocation`) :`false` (`self.CubeLocationA`) :`true` (`self.CubeLocationB`)))))

(fn `UserConstructionScript`
  (`parent.UserConstructionScript`))
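; BP_Dare is the Dare car Blueprint, a child class that adds fire and explosion effects when the car crashes.
; Its HandleCrash event runs the parent crash logic, then activates the Fire and FireSFX components without resetting them.
; It then spawns an explosion particle at the car's location and plays the explosion sound at the impact point.
; The construction script only calls the parent.
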(event `self.HandleCrash`
  (params (Hit :type "HitResult Structure (by ref)"))
  (`|ExecutionSequence`
    (:`then_0`
      (`parent.HandleCrash` Hit))
    (:`then_1`
      (`ActorComponent.Activate` (`self.Fire`) false))
    (:`then_2`
      (`ActorComponent.Activate` (`self.FireSFX`) false))
    (:`then_3`
      (`GameplayStatics.SpawnEmitterAtLocation` "/Game/StarterContent/Particles/P_Explosion.P_Explosion" (`self.K2_GetActorLocation`))
      (`GameplayStatics.PlaySoundAtLocation` "/Game/StarterContent/Audio/Explosion_Cue.Explosion_Cue" (`.Location` (`GameplayStatics.BreakHitResult` Hit))))))

(fn `UserConstructionScript`
  (`parent.UserConstructionScript`))